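; Scrolling building-and-road scenery segment for a driving game that moves itself each tick, swaps materials by player Modo and can spawn a successor.
; When Started, it shows a left or right Civic obstacle based on the player's FezCurvaE.
; Obstacle triggers set slow Speed on all segments and open BP_Puzzle widgets.
; End triggers read AcertouTudo, then restore speeds, close the puzzle and call CurvaE on success; life-loss logic is unwired.
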(event OnComponentBeginOverlap(ObstaculoD)
  (params (OverlappedComponent :type Primitive%20Component%20Object%20Reference) (OtherActor :type Actor%20Object%20Reference) (OtherComp :type Primitive%20Component%20Object%20Reference) (OtherBodyIndex :type Integer) (bFromSweep :type Boolean) (SweepResult :type Hit%20Result%20Structure%20%28by%20ref%29))
  (if (Variables|Default|GetCriarObstaculoD)
    (bind _asbp_carro_player (Utilities|Casting|CastToBP_CarroPlayer OtherActor))
    (if (Variables|/Game/Player/BP_CarroPlayer.BP_CarroPlayer_C|GetFezCurvaE _asbp_carro_player)
      (Variables|/Game/Player/BP_CarroPlayer.BP_CarroPlayer_C|SetFezCurvaE _asbp_carro_player false))
    (Variables|/Game/Player/BP_CarroPlayer.BP_CarroPlayer_C|SetVelocidadeRodas _asbp_carro_player 5.0)
    (bind _outactors (Actor|GetAllActorsOfClass "BP_CenarioPredios_C"))
    (for _array_element _outactors
      (Variables|BP_CenarioPredios_C|SetSpeed _array_element -1.0)
      (Utilities|FlowControl|Delay 0.1)
      (bind _returnvalue (UserInterface|CreateWidget "/Game/HUD/BP_Puzzle.BP_Puzzle_C"))
      (bind _output_get (Variables|Default|SetHudPuzzle _returnvalue))
      (UserInterface|Viewport|AddtoViewport _output_get 0))))

(event OnComponentBeginOverlap(FimObstaculoD)
  (params (OverlappedComponent :type Primitive%20Component%20Object%20Reference) (OtherActor :type Actor%20Object%20Reference) (OtherComp :type Primitive%20Component%20Object%20Reference) (OtherBodyIndex :type Integer) (bFromSweep :type Boolean) (SweepResult :type Hit%20Result%20Structure%20%28by%20ref%29))
  (if (Variables|Default|GetCriarObstaculoD)
    (bind _asbp_puzzle (Utilities|Casting|CastToBP_Puzzle (Variables|Default|GetHudPuzzle)))
    (Variables|Default|SetAcertouTudo (Variables|/Game/HUD/BP_Puzzle.BP_Puzzle_C|GetAcertouTudo _asbp_puzzle))))

(event OnComponentBeginOverlap(ObstaculoE)
  (params (OverlappedComponent :type Primitive%20Component%20Object%20Reference) (OtherActor :type Actor%20Object%20Reference) (OtherComp :type Primitive%20Component%20Object%20Reference) (OtherBodyIndex :type Integer) (bFromSweep :type Boolean) (SweepResult :type Hit%20Result%20Structure%20%28by%20ref%29))
  (if (Variables|Default|GetCriarObstaculoE)
    (bind _asbp_carro_player (Utilities|Casting|CastToBP_CarroPlayer OtherActor))
    (if (Variables|/Game/Player/BP_CarroPlayer.BP_CarroPlayer_C|GetFezCurvaE _asbp_carro_player)
      _
      (else
        (Variables|/Game/Player/BP_CarroPlayer.BP_CarroPlayer_C|SetFezCurvaE _asbp_carro_player true)))
    (Variables|/Game/Player/BP_CarroPlayer.BP_CarroPlayer_C|SetVelocidadeRodas _asbp_carro_player 5.0)
    (bind _outactors (Actor|GetAllActorsOfClass "BP_CenarioPredios_C"))
    (for _array_element _outactors
      (Variables|BP_CenarioPredios_C|SetSpeed _array_element -1.0)
      (Utilities|FlowControl|Delay 0.1)
      (bind _returnvalue (UserInterface|CreateWidget "/Game/HUD/BP_Puzzle.BP_Puzzle_C"))
      (bind _output_get (Variables|Default|SetHudPuzzle _returnvalue))
      (UserInterface|Viewport|AddtoViewport _output_get 0))))

(event OnComponentBeginOverlap(FimObstaculoE)
  (params (OverlappedComponent :type Primitive%20Component%20Object%20Reference) (OtherActor :type Actor%20Object%20Reference) (OtherComp :type Primitive%20Component%20Object%20Reference) (OtherBodyIndex :type Integer) (bFromSweep :type Boolean) (SweepResult :type Hit%20Result%20Structure%20%28by%20ref%29))
  (if (Variables|Default|GetCriarObstaculoE)
    (bind _asbp_puzzle (Utilities|Casting|CastToBP_Puzzle (Variables|Default|GetHudPuzzle)))
    (Variables|Default|SetAcertouTudo (Variables|/Game/HUD/BP_Puzzle.BP_Puzzle_C|GetAcertouTudo _asbp_puzzle))))

(event OnComponentBeginOverlap(FimObstaculoDFechaTela)
  (params (OverlappedComponent :type Primitive%20Component%20Object%20Reference) (OtherActor :type Actor%20Object%20Reference) (OtherComp :type Primitive%20Component%20Object%20Reference) (OtherBodyIndex :type Integer) (bFromSweep :type Boolean) (SweepResult :type Hit%20Result%20Structure%20%28by%20ref%29))
  (if (Variables|Default|GetCriarObstaculoD)
    (CallFunction|FechaTelaPuzzle)))

(event OnComponentBeginOverlap(FimObstaculoEFechaTela)
  (params (OverlappedComponent :type Primitive%20Component%20Object%20Reference) (OtherActor :type Actor%20Object%20Reference) (OtherComp :type Primitive%20Component%20Object%20Reference) (OtherBodyIndex :type Integer) (bFromSweep :type Boolean) (SweepResult :type Hit%20Result%20Structure%20%28by%20ref%29))
  (if (Variables|Default|GetCriarObstaculoE)
    (CallFunction|FechaTelaPuzzle)))

(event Custom|SpawnNext
  (if (Variables|Default|GetSpawn?)
    (Variables|Default|SetSpawned true)
    (Utilities|FlowControl|Delay 0.2)
    (bind _returnvalue (Game|SpawnActorfromClass "BP_CenarioPredios_C" (Transformation|GetWorldTransform (Variables|Default|GetScene)) "AlwaysSpawn" 0 0))
    (Variables|BP_CenarioPredios_C|SetSpeed _returnvalue (Variables|Default|GetSpeed))
    (Variables|BP_CenarioPredios_C|SetSpawnedRef _returnvalue 0)))

(event Custom|VisibilidadeObstaculo
  (if (Variables|Default|GetCriarObstaculoD)
    (Rendering|SetVisibility (Variables|Default|GetCivicD) true false)
    (Rendering|SetVisibility (Variables|Default|GetRodaCivic1) true false)
    (Rendering|SetVisibility (Variables|Default|GetRodaCivic2) true false)
    (Rendering|SetVisibility (Variables|Default|GetRodaCivic3) true false)
    (else
      (Rendering|SetVisibility (Variables|Default|GetCivicE) true false)
      (Rendering|SetVisibility (Variables|Default|GetRodaCivic4) true false)
      (Rendering|SetVisibility (Variables|Default|GetRodaCivic5) true false)
      (Rendering|SetVisibility (Variables|Default|GetRodaCivic6) true false))))

(event Custom|FechaTelaPuzzle
  (bind _hudpuzzle (Variables|Default|GetHudPuzzle))
  (bind _outactors (Actor|GetAllActorsOfClass "/Game/Player/BP_CarroPlayer.BP_CarroPlayer_C"))
  (bind _asbp_carro_player (Utilities|Casting|CastToBP_CarroPlayer (Utilities|Array|Get(acopy) _outactors)))
  (Variables|/Game/Player/BP_CarroPlayer.BP_CarroPlayer_C|SetVelocidadeRodas _asbp_carro_player 2e+01)
  (Variables|/Game/Player/BP_CarroPlayer.BP_CarroPlayer_C|SetVelocidadeMapa_0 _asbp_carro_player -1e+01)
  (Default|DespausaSom _asbp_carro_player)
  (bind _asbp_hud_2 (Utilities|Casting|CastToBP_Hud2 (Variables|/Game/Player/BP_CarroPlayer.BP_CarroPlayer_C|GetHUD _asbp_carro_player)))
  (Variables|/Game/HUD/BP_Hud2.BP_Hud2_C|Setpuzzle? _asbp_hud_2 false)
  (bind _outactors_2 (Actor|GetAllActorsOfClass "BP_CenarioPredios_C"))
  (for _array_element _outactors_2
    (Variables|BP_CenarioPredios_C|SetSpeed _array_element -1e+01)
    (Utilities|IsValid _hudpuzzle
      (:Is%20Valid
        (Widget|RemovefromParent _hudpuzzle))
      (:Is%20Not%20Valid
        _))
    (if (Variables|Default|GetAcertouTudo)
      (Utilities|FlowControl|Delay 0.1)
      (bind _returnvalue (Actor|GetActorOfClass "/Game/Player/BP_CarroPlayer.BP_CarroPlayer_C"))
      (Default|CurvaE _returnvalue))))

(event EventBeginPlay
  (Variables|Default|SetVelocidade -1e+01)
  (if (Variables|Default|GetStarted?)
    (bind _outactors (Actor|GetAllActorsOfClass "/Game/Player/BP_CarroPlayer.BP_CarroPlayer_C"))
    (if (Variables|/Game/Player/BP_CarroPlayer.BP_CarroPlayer_C|GetFezCurvaE (Utilities|Array|Get(acopy) _outactors))
      (Variables|Default|SetCriarObstaculoE true)
      (else
        (Variables|Default|SetCriarObstaculoD true)))
    (CallFunction|VisibilidadeObstaculo)))

(event EventTick
  (params (DeltaSeconds :type Float%20%28single-precision%29))
  (Transformation|AddWorldOffset (Variables|Default|GetDefaultSceneRoot) (Math|Vector|MakeVector 0.0 (Variables|Default|GetVelocidade) 0.0) false false)
  (bind _outactors (Actor|GetAllActorsOfClass "/Game/Player/BP_CarroPlayer.BP_CarroPlayer_C"))
  (if (not (== (Variables|/Game/Player/BP_CarroPlayer.BP_CarroPlayer_C|GetModo (Utilities|Array|Get(acopy) _outactors)) 0))
    (Rendering|Material|SetMaterial (Variables|Default|GetStaticMesh) 0 "/Game/Cenario/Fundo/FundoMaterial1.FundoMaterial1")
    (Rendering|Material|SetMaterial (Variables|Default|GetStaticMesh2) 0 "/Game/Cenario/Fundo/FundoMaterial1.FundoMaterial1")
    (Rendering|Material|SetMaterial (Variables|Default|GetRua) 0 0)))

(fn ConstructionScript)