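; BP_CenarioSpawner is an actor that triggers continuous spawning of scenery segments and places puzzle obstacles for the player car.
; Each Tick it line-traces downward for a BP_CenarioPredios tile, caching it if already spawned, otherwise calling SpawnNext.
; After that spawn, when started, in car mode 0 and with AtivarPuzzle on, it enables a left or right obstacle based on the car's FezCurvaE turn flag.
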(event EventBeginPlay)

(event Collision|EventActorBeginOverlap
  (params (OtherActor :type Actor%20Object%20Reference)))

(event EventTick
  (params (DeltaSeconds :type Float%20%28single-precision%29))
  (bind _defaultsceneroot (Variables|Default|GetDefaultSceneRoot))
  (bind _returnvalue (Transformation|GetWorldLocation _defaultsceneroot))
  (bind _outhit (Collision|LineTraceByChannel _returnvalue (+ _returnvalue "0, 0,-100.000000") "TraceTypeQuery1" true 0 "None" true "(R=1.000000,G=0.000000,B=0.000000,A=1.000000)" "(R=0.000000,G=1.000000,B=0.000000,A=1.000000)" 1.0))
  (bind _asbp_cenario_predios (Utilities|Casting|CastToBP_CenarioPredios (.hitactor _outhit)))
  (if (Variables|/Game/Cenario/BP_CenarioPredios.BP_CenarioPredios_C|GetSpawned _asbp_cenario_predios)
    (Variables|Default|SetBP_Cenario _asbp_cenario_predios)
    (else
      (Default|SpawnNext _asbp_cenario_predios)
      (if (Variables|Default|GetStarted)
        (bind _outactors (Actor|GetAllActorsOfClass "/Game/Player/BP_CarroPlayer.BP_CarroPlayer_C"))
        (if (== (Variables|/Game/Player/BP_CarroPlayer.BP_CarroPlayer_C|GetModo (Utilities|Array|Get(acopy) _outactors)) 0)
          (if (Variables|Default|GetAtivarPuzzle)
            (bind _outactors_2 (Actor|GetAllActorsOfClass "/Game/Player/BP_CarroPlayer.BP_CarroPlayer_C"))
            (if (Variables|/Game/Player/BP_CarroPlayer.BP_CarroPlayer_C|GetFezCurvaE (Utilities|Array|Get(acopy) _outactors_2))
              (Variables|/Game/Cenario/BP_CenarioPredios.BP_CenarioPredios_C|SetCriarObstaculoE _asbp_cenario_predios true)
              (else
                (Variables|/Game/Cenario/BP_CenarioPredios.BP_CenarioPredios_C|SetCriarObstaculoD _asbp_cenario_predios true)))
            (Default|VisibilidadeObstaculo _asbp_cenario_predios)))))))

(fn ConstructionScript)