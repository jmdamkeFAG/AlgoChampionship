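; Game mode that holds answer-checking helpers for the game's puzzles, backed by the DT_Puzzles data table.
; ValidarResposta looks up a puzzle row by ID and compares user answers to RespostasCorretas by index, returning a per-answer boolean array.
; ValidarSeAcertou, despite its name, only returns the correct-answer count and an empty Respostas value.
; Event graph and construction script are empty.
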(event EventBeginPlay)

(event EventTick
  (params (DeltaSeconds :type Float%20%28single-precision%29)))

(fn ConstructionScript)

(fn ValidarResposta
  (params (ID_Puzzle :type Name) (Respostas_Usuarios :type Array%20of%20Strings))
  (bind _returnvalue (Utilities|GetDataTableRow "/Game/DT_Puzzles.DT_Puzzles" ID_Puzzle)
    (:then
      (Utilities|Array|Clear (Variables|Default|GetResultadosTemp))
      (for (_array_element _array_index) (.RespostasCorretas (Utilities|Struct|BreakS_PuzzleQuestao _returnvalue))
        (Utilities|Array|Add (Variables|Default|GetResultadosTemp) (Utilities|Enum|Equal(Enum) (Utilities|Array|Get(acopy) Respostas_Usuarios _array_index) _array_element)))
      (return (Variables|Default|GetResultadosTemp)))))

(fn ValidarSeAcertou
  (params (ID_Puzzle :type Name))
  (bind _returnvalue (Utilities|GetDataTableRow "/Game/DT_Puzzles.DT_Puzzles" ID_Puzzle)
    (:then
      (return (Utilities|Array|Length (.RespostasCorretas (Utilities|Struct|BreakS_PuzzleQuestao _returnvalue))) ""))))