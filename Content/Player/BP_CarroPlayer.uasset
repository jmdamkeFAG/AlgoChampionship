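; Player car for a racing game that stays in place along the track while wheel spin and scenery speed simulate driving.
; StartRace runs the countdown and HUD, and gear engine sounds act as the race clock, feeding gear progress and advancing on finish.
; In mode 1, gear changes trigger slow motion and a puzzle, then a win screen.
; Timelines animate launch, lane swaps and wheel shake; losing health blinks the car.
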(event OnAudioFinished(Audio)
  (bind _marchaatual (Variables|Default|GetMarchaAtual))
  (if (>= (Variables|Default|GetMarchaAtual) 5)
    (if (== (Variables|Default|GetModo) 0)
      _
      (else
        (Math|Integer|IncrementInt (Variables|Default|GetMarchaAtual) :!label _label
          (:%20%20
            _))))
    (else
      (goto _label)))
  (bind _asbp_hud_2 (Utilities|Casting|CastToBP_Hud2 (Variables|Default|GetHUD))
    (:then
      (Variables|/Game/HUD/BP_Hud2.BP_Hud2_C|SetMarcha _asbp_hud_2 (Variables|Default|GetMarchaAtual)))
    (:CastFailed
      _))
  (CallFunction|TocarSomMarcha)
  (if (== (Variables|Default|GetModo) 1)
    (if (> _marchaatual 1)
      (if (> _marchaatual 5)
        (Game|SetGamePaused true)
        (bind _returnvalue (UserInterface|CreateWidget "/Game/HUD/BP_End_Game.BP_End_Game_C"))
        (Default|Win _returnvalue)
        (UserInterface|Viewport|AddtoViewport _returnvalue 0)
        (else
          (CallFunction|CameraLenta)
          (CallFunction|PausaSom)
          (bind _returnvalue_2 (UserInterface|CreateWidget "/Game/HUD/BP_Puzzle.BP_Puzzle_C"))
          (UserInterface|Viewport|AddtoViewport _returnvalue_2 0))))))

(event OnAudioFinished(Audio1)
  (bind _audio1 (Variables|Default|GetAudio1))
  (Audio|Components|Audio|SetSound _audio1 "/Game/Musics/Marchas/motorloop.motorloop")
  (Audio|Components|Audio|Play _audio1 0.0))

(event Custom|CurvaE
  (if (Variables|Default|GetFezCurvaE)
    (CallFunction|CurvaD)
    (else
      (Variables|Default|SetFezCurvaE true)
      (bind (_direction _suspensaoy _localpista) (Timeline|CurvaEsquerda PlayFromStart)
        (:Update
          (Transformation|SetRelativeRotation (Variables|Default|GetStaticMesh) (Math|Rotator|MakeRotator (* _suspensaoy -0.3) _suspensaoy (* _suspensaoy -2.0)) false false)
          (Transformation|SetRelativeRotation (Variables|Default|GetScene) (Math|Rotator|MakeRotator 0.0 0.0 (* _suspensaoy -2.0)) false false)
          (Transformation|SetWorldLocation (Variables|Default|GetDefaultSceneRoot) (Math|Vector|MakeVector _localpista 9077.0 7e+01) false false))))))

(event Custom|CurvaD
  (Variables|Default|SetFezCurvaE false)
  (bind (_direction _suspensaoy _localpista _localpistad) (Timeline|Timeline_0 PlayFromStart)
    (:Update
      (Transformation|SetRelativeRotation (Variables|Default|GetStaticMesh) (Math|Rotator|MakeRotator (* _suspensaoy -0.3) (* _suspensaoy -1.0) (* _suspensaoy 2.0)) false false)
      (Transformation|SetRelativeRotation (Variables|Default|GetScene) (Math|Rotator|MakeRotator 0.0 0.0 (* _suspensaoy 2.0)) false false)
      (Transformation|SetWorldLocation (Variables|Default|GetDefaultSceneRoot) (Math|Vector|MakeVector _localpistad 9077.0 7e+01) false false))))

(event Custom|PerdeuVida
  (Math|Integer|DecrementInt (Variables|Default|GetSaudeDoCarro)
    (:%20%20
      (bind _asbp_hud_2 (Utilities|Casting|CastToBP_Hud2 (Variables|Default|GetHUD)))
      (Default|PerdeuVida _asbp_hud_2)
      (if (== (Variables|Default|GetModo) 0)
        (Utilities|FlowControl|Delay 0.8))
      (CallFunction|Pisca))))

(event Custom|StartRace
  (Variables|Default|SetAcertos 0)
  (CallFunction|TocarSomMarcha)
  (Variables|Default|SetVelocidadeRodas 0.0)
  (bind _outactors (Actor|GetAllActorsOfClass "/Game/Cenario/BP_CenarioSpawner.BP_CenarioSpawner_C"))
  (Variables|/Game/Cenario/BP_CenarioSpawner.BP_CenarioSpawner_C|SetStarted (Utilities|Array|Get(acopy) _outactors) true)
  (Variables|Default|SetVelocidadeMapa -1e+01)
  (bind _returnvalue (UserInterface|CreateWidget "/Game/HUD/BP_Contagem.BP_Contagem_C"))
  (UserInterface|Viewport|AddtoViewport _returnvalue 0)
  (Utilities|FlowControl|Delay 2.2)
  (Rendering|Components|TextRender|SetText (Variables|/Game/HUD/BP_Contagem.BP_Contagem_C|GetTextBlock_0 _returnvalue) "2")
  (Utilities|FlowControl|Delay 1.0)
  (Rendering|Components|TextRender|SetText (Variables|/Game/HUD/BP_Contagem.BP_Contagem_C|GetTextBlock_0 _returnvalue) "1")
  (Utilities|FlowControl|Delay 1.0)
  (Rendering|Components|TextRender|SetText (Variables|/Game/HUD/BP_Contagem.BP_Contagem_C|GetTextBlock_0 _returnvalue) "Vai!")
  (Utilities|FlowControl|Delay 1.0)
  (Widget|RemovefromParent (Variables|/Game/HUD/BP_Contagem.BP_Contagem_C|GetTextBlock_0 _returnvalue))
  (Variables|Corrida|SetIdle? false)
  (Variables|Corrida|SetCorridaComecou true)
  (Widget|RemovefromParent (Variables|Default|GetMenu))
  (bind _returnvalue_2 (UserInterface|CreateWidget "/Game/HUD/BP_Hud2.BP_Hud2_C"))
  (Variables|Default|SetHUD _returnvalue_2)
  (UserInterface|Viewport|AddtoViewport _returnvalue_2 0)
  (bind _saida (Timeline|Saida PlayFromStart)
    (:Update
      (Transformation|SetRelativeRotation (Variables|Default|GetStaticMesh) (Math|Rotator|MakeRotator (* _saida -1.7) 0.0 0.0) false false))))

(event Custom|Pisca
  (Utilities|FlowControl|FlipFlop
    (:A
      (Rendering|SetVisibility (Variables|Default|GetStaticMesh) false false)
      (for _array_element (Variables|Default|GetRodas)
        (Rendering|SetVisibility _array_element false false)
        (Utilities|FlowControl|Delay 0.1)
        (CallFunction|Pisca)))
    (:B
      (Rendering|SetVisibility (Variables|Default|GetStaticMesh) true false)
      (for _array_element_2 (Variables|Default|GetRodas)
        (Rendering|SetVisibility _array_element_2 true false)
        (Utilities|FlowControl|Delay 0.1)
        (bind _result (Math|Integer|IncrementInt (Variables|Default|GetPiscadas))
          (:%20%20
            (if (> _result 4)
              (Variables|Default|SetPiscadas 0)
              (else
                (CallFunction|Pisca)))))))))

(event Custom|CameraLenta
  (Variables|Default|SetVelocidadeSaida 1e+02)
  (Variables|Default|SetVelocidadeRodas 2.0)
  (Variables|Default|SetVelocidadeMapa_0 -1.0))

(event Custom|CameraNormal
  (Variables|Default|SetVelocidadeSaida 0.3)
  (Variables|Default|SetVelocidadeRodas 2e+01)
  (Variables|Default|SetVelocidadeMapa_0 -1e+01))

(event Custom|TocarSomMarcha
  (bind _audio (Variables|Default|GetAudio))
  (switch int (Variables|Default|GetMarchaAtual)
    (:0
      (Audio|Components|Audio|SetSound _audio "/Game/Musics/Marchas/motor_ligando.motor_ligando"))
    (:1
      (Audio|Components|Audio|SetSound _audio "/Game/Musics/Marchas/motor_primeira_marcha.motor_primeira_marcha"))
    (:2
      (Audio|Components|Audio|SetSound _audio "/Game/Musics/Marchas/motor_segunda_marcha.motor_segunda_marcha"))
    (:3
      (Audio|Components|Audio|SetSound _audio "/Game/Musics/Marchas/motor_terceira_marcha.motor_terceira_marcha"))
    (:4
      (Audio|Components|Audio|SetSound _audio "/Game/Musics/Marchas/motor_quarta_marcha.motor_quarta_marcha"))
    (:5
      (Audio|Components|Audio|SetSound _audio "/Game/Musics/Marchas/motor_quinta_marcha_continua.motor_quinta_marcha_continua" :!label _label))
    (:6
      (goto _label)))
  (Audio|Components|Audio|Play _audio 0.0)
  (Variables|Default|SetDuracaoTotalMarcha (Variables|/Script/Engine.SoundBase|GetDuration (Variables|/Script/Engine.AudioComponent|GetSound _audio)))
  (Variables|Default|SetTempoDecorrido 0.0))

(event Custom|PausaSom
  (Class|AudioComponent|SetPaused (Variables|Default|GetAudio) true))

(event Custom|DespausaSom
  (Class|AudioComponent|SetPaused (Variables|Default|GetAudio) false))

(event EventBeginPlay
  (Variables|Default|SetVelocidadeRodas 2e+01)
  (bind _outactors (Actor|GetAllActorsOfClass "/Game/Cenario/BP_CenarioPredios.BP_CenarioPredios_C"))
  (Variables|/Game/Cenario/BP_CenarioPredios.BP_CenarioPredios_C|SetSpeed (Utilities|Array|Get(acopy) _outactors) -1e+01)
  (bind _returnvalue (UserInterface|CreateWidget "/Game/HUD/BP_Menu.BP_Menu_C"))
  (bind _output_get (Variables|Default|SetMenu _returnvalue))
  (UserInterface|Viewport|AddtoViewport _output_get 0)
  (bind _variacao (Timeline|TremorRodas Play)
    (:Update
      (for _array_element (Variables|Default|GetRodas)
        (if (> (Variables|Default|GetVelocidadeRodas) 5.0)
          (Transformation|SetRelativeLocation _array_element (+ (Variables|/Script/Engine.SceneComponent|GetRelativeLocation _array_element) (Math|Vector|MakeVector 0.0 0.0 (* _variacao (Math|Random|RandomFloatinRange 0.0 0.08)))) false false)
          (Utilities|FlowControl|Delay 0.2)
          (for (_array_element_2 _array_index) (Variables|Default|GetRodas)
            (Transformation|SetRelativeLocation _array_element_2 (Utilities|Array|Get(acopy) (Variables|Default|GetRodasPosicao) _array_index) false false)))))))

(event EventTick
  (params (DeltaSeconds :type Float%20%28single-precision%29))
  (bind _output_get (Variables|Default|SetDeltaSeconds DeltaSeconds))
  (Utilities|FlowControl|Sequence
    (:then_0
      (if (Variables|Corrida|GetCorridaComecou)
        (Variables|Default|SetVelocidadeRodas (Math|Interpolation|FInterpTo (Variables|Default|GetVelocidadeRodas) (Variables|Default|GetVelocidadeCarro) (Variables|Default|GetDeltaSeconds) (Variables|Default|GetVelocidadeSaida)))
        (bind _outactors (Actor|GetAllActorsOfClass "/Game/Cenario/BP_CenarioPredios.BP_CenarioPredios_C"))
        (for _array_element _outactors
          (Variables|/Game/Cenario/BP_CenarioPredios.BP_CenarioPredios_C|SetVelocidade _array_element (Math|Interpolation|FInterpTo (Variables|/Game/Cenario/BP_CenarioPredios.BP_CenarioPredios_C|GetVelocidade _array_element) (Variables|Default|GetVelocidadeMapa_0) (Variables|Default|GetDeltaSeconds) (Variables|Default|GetVelocidadeSaida))))
        (for _array_element_2 (Variables|Default|GetRodas) :!label _label
          (Transformation|AddLocalRotation _array_element_2 (Math|Rotator|MakeRotator (Variables|Default|GetVelocidadeRodas) 0.0 0.0) false false))
        (if (Variables|Corrida|GetCorridaComecou)
          (if (not (Variables|Corrida|GetCorridaAcabou))
            (Variables|Corrida|SetTempoAtual (+ (Variables|Corrida|GetTempoAtual) (Utilities|Time|GetWorldDeltaSeconds)))))
        (elif (Variables|Corrida|GetIdle?)
          (goto _label))))
    (:then_1
      (if (Audio|Components|Audio|IsPlaying (Variables|Default|GetAudio))
        (bind _output_get_2 (Variables|Default|SetTempoDecorrido (+ (Variables|Default|GetTempoDecorrido) _output_get)))
        (bind _asbp_hud_2 (Utilities|Casting|CastToBP_Hud2 (Variables|Default|GetHUD)))
        (Variables|/Game/HUD/BP_Hud2.BP_Hud2_C|Setvalor _asbp_hud_2 (/ _output_get_2 (Variables|Default|GetDuracaoTotalMarcha)))))))

(fn ConstructionScript
  (Utilities|Array|Add (Variables|Default|GetRodas) (Variables|Default|GetRodaTE))
  (Utilities|Array|Add (Variables|Default|GetRodas) (Variables|Default|GetRodaFE))
  (Utilities|Array|Add (Variables|Default|GetRodas) (Variables|Default|GetRodaFD))
  (Utilities|Array|Add (Variables|Default|GetRodas) (Variables|Default|GetRodaTD)))